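; BP_Token is a placeable game piece for a turn-based board game with win and draw conditions.
; Its Sphere overlaps track the current BP_Slot, coloring it on entry and resetting it to GroundColor on exit.
; Lockin accepts one placement on a valid slot, moves the mesh there and makes it Stationary.
; It then queries BP_WinningCondition and, without a win or draw, tells ThirdPersonGameMode to change player.
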(event OnComponentBeginOverlap(Sphere)
  (params (OverlappedComponent :type Primitive%20Component%20Object%20Reference) (OtherActor :type Actor%20Object%20Reference) (OtherComp :type Primitive%20Component%20Object%20Reference) (OtherBodyIndex :type Integer) (bFromSweep :type Boolean) (SweepResult :type Hit%20Result%20Structure%20%28by%20ref%29))
  ;[1 1 1] Color The Planes (Slot)
  (if (== (Utilities|GetClass OtherActor) "/Game/BluePrints/BP_Slot.BP_Slot_C")
    (Variables|Default|SetSlot OtherActor)
    (Class|IFSlot|SetColor(Message) OtherActor (Variables|Default|GetColor) (Game|Player|GetPlayerPawn 0))
    (Variables|Default|SetValidSlot true)))

(event OnComponentEndOverlap(Sphere)
  (params (OverlappedComponent :type Primitive%20Component%20Object%20Reference) (OtherActor :type Actor%20Object%20Reference) (OtherComp :type Primitive%20Component%20Object%20Reference) (OtherBodyIndex :type Integer))
  ;[1 1 1] Reset color on slots
  (if (== (Variables|Default|GetSlot) OtherActor)
    (if (== (Utilities|GetClass OtherActor) "/Game/BluePrints/BP_Slot.BP_Slot_C")
      (Class|IFSlot|SetColor(Message) OtherActor (Variables|Default|GetGroundColor))
      (Variables|Default|SetValidSlot false))))

(event EventLockin
  ;[1 1 1] LockToken in Valid Position
  (if (Variables|Default|GetValidSlot)
    (if (Variables|Default|GetLocked)
      (Development|PrintString "Already placed Token")
      (else
        (Default|CallLockToken)
        (Audio|PlaySoundatLocation "/Game/StarterContent/Audio/Sci_Fi_Door_Opening_or_Closing.Sci_Fi_Door_Opening_or_Closing" (Transformation|GetActorLocation) "0, 0, 0" 1.0 1.0 0.5 0 0 0)
        (Variables|Default|SetLocked true)
        (Transformation|SetRelativeLocationAndRotation (Variables|Default|GetStaticMesh) (Transformation|GetActorLocation (Variables|Default|GetSlot)) "0,45.000000, 0" false false)
        (Transformation|SetMobility (Variables|Default|GetStaticMesh) "Stationary")
        (bind _returnvalue (Actor|GetActorOfClass "/Game/BluePrints/BP_WinningCondition.BP_WinningCondition_C"))
        (bind _won (Default|Winning _returnvalue))
        (if (not _won)
          (bind _draw (Default|Draw _returnvalue))
          (if (not _draw)
            (bind _returnvalue_2 (Actor|GetActorOfClass "/Game/ThirdPersonBP/Blueprints/ThirdPersonGameMode.ThirdPersonGameMode_C"))
            (Default|ChangePlayer _returnvalue_2)))))
    (else
      (Development|PrintString "Token not in valid positon"))))

(fn ConstructionScript)