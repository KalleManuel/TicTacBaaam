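; Trigger-box actor that repeatedly reports the Speed stat through BP_PlayerStats while its overlap timer runs.
; Begin overlap, gated by a negated owner comparison against ThirdPersonCharacter, finds BP_PlayerStats and starts a looping timer.
; Each SpeedBoost tick passes the current Speed value to StatsMessage without changing it here.
; End overlap clears the timer only when the leaving actor casts to ThirdPersonCharacter.
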(event OnComponentBeginOverlap(Box)
  (params (OverlappedComponent :type Primitive%20Component%20Object%20Reference) (OtherActor :type Actor%20Object%20Reference) (OtherComp :type Primitive%20Component%20Object%20Reference) (OtherBodyIndex :type Integer) (bFromSweep :type Boolean) (SweepResult :type Hit%20Result%20Structure%20%28by%20ref%29))
  (if (not (== (Components|GetOwner OtherActor) "/Game/ThirdPersonBP/Blueprints/ThirdPersonCharacter.ThirdPersonCharacter"))
    (bind _returnvalue (Actor|GetActorOfClass "/Game/BluePrints/BP_PlayerStats.BP_PlayerStats_C"))
    (bind _returnvalue_2 (Utilities|Time|SetTimerbyEvent (delegate Custom|SpeedBoost) 2.0 true))
    (Variables|Default|SetBoostTimer _returnvalue_2)))

(event OnComponentEndOverlap(Box)
  (params (OverlappedComponent :type Primitive%20Component%20Object%20Reference) (OtherActor :type Actor%20Object%20Reference) (OtherComp :type Primitive%20Component%20Object%20Reference) (OtherBodyIndex :type Integer))
  (Utilities|Casting|CastToThirdPersonCharacter OtherActor)
  (Utilities|Time|ClearandInvalidateTimerbyHandle (Variables|Default|GetBoostTimer)))

(event Custom|SpeedBoost
  (Class|IFStats|Stats(Message) (stale OnComponentBeginOverlap(Box) _returnvalue) (Variables|/Game/BluePrints/BP_PlayerStats.BP_PlayerStats_C|GetSpeed (stale OnComponentBeginOverlap(Box) _returnvalue)) (Utilities|Name|MakeLiteralName "Speed")))

(fn ConstructionScript)