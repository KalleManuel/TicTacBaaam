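; BP_PlayerStats is an actor that holds the player's Speed, Strength, Shield and Radius stats along with their money.
; On BeginPlay it totals the stats into TotalPower, sets starting Dollars and creates the HUD.
; The Stats event buys a boost by stat name, limited by cost, a per-stat cap and a TotalPower cap; Radius boosts also notify ThirdPersonCharacter.
; WinDollar and DrawDollar events add match rewards to Dollars.
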(event Custom|WinDollar
  (Variables|Default|SetDollars (+ (Variables|Default|GetDollars) (Variables|Default|GetWinMoney))))

(event Custom|DrawDollar
  (Variables|Default|SetDollars (+ (Variables|Default|GetDollars) (Variables|Default|GetDrawMoney))))

(event EventStats
  (params (CurrentStat :type Float%20%28single-precision%29) (StatName :type Name :default "None"))
  (if (not (>= CurrentStat 1e+01))
    (if (>= (Variables|Default|GetDollars) (Variables|Default|GetBoostCost))
      (if (< (Variables|Default|GetTotalPower) 2e+01)
        (Variables|Default|SetTotalPower (+ (Variables|Default|GetTotalPower) 1.0))
        (Variables|Default|SetDollars (- (Variables|Default|GetDollars) (Variables|Default|GetBoostCost)))
        (if (== StatName "Speed")
          (Variables|Default|SetSpeed (+ (Variables|Default|GetSpeed) (Variables|Default|GetBoostAmount)))
          (elif (== StatName "Strength")
            (Variables|Default|SetStrength (+ (Variables|Default|GetStrength) (Variables|Default|GetBoostAmount)))
            (elif (== StatName "Shield")
              (Variables|Default|SetShield (+ (Variables|Default|GetShield) (Variables|Default|GetBoostAmount)))
              (elif (== StatName "Radius")
                (Variables|Default|SetRadius (+ (Variables|Default|GetRadius) (Variables|Default|GetBoostAmount)))
                (bind _returnvalue (Actor|GetActorOfClass "/Game/ThirdPersonBP/Blueprints/ThirdPersonCharacter.ThirdPersonCharacter_C"))
                (Default|AddtoRadius _returnvalue)))))))))

(event EventBeginPlay
  (Variables|Default|SetTotalPower (+ (Variables|Default|GetTotalPower) (Variables|Default|GetSpeed) (Variables|Default|GetStrength) (Variables|Default|GetShield) (Variables|Default|GetRadius)))
  (Variables|Default|SetDollars (Variables|Default|GetDollarsToStartWith))
  (bind _returnvalue (UserInterface|CreateWidget "/Game/Widgets/HUD/HUD.HUD_C"))
  (UserInterface|Viewport|AddtoViewport _returnvalue 0))

(fn ConstructionScript)