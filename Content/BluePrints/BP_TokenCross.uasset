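; BP_TokenCross is a cross token actor that is destroyed on timeout unless it has been locked in place.
; On BeginPlay it binds to the ThirdPersonGameMode destroy-token dispatcher and its own lock dispatcher, then plays an impact sound after a short delay.
; The lock event sets LockedCross, which makes the token ignore the destroy broadcast.
; An unlocked token spawns an explosion effect and sound before destroying itself.
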(event Custom|Destroy%20Token
  (bind _returnvalue (Transformation|GetActorLocation))
  ;[1 1 1] Destroy token if times up
  (if (not (Variables|Default|GetLockedCross))
    (Effects|SpawnEmitteratLocation "/Game/StarterContent/Particles/P_Explosion.P_Explosion" _returnvalue "0, 0, 0" "2.000000,2.000000,2.000000")
    (Audio|PlaySoundatLocation "/Game/StarterContent/Audio/Explosion02.Explosion02" _returnvalue "0, 0, 0" 1.0 1.0 0.0 0 0 0)
    (Actor|DestroyActor)))

(event Custom|Lock%20This%20token
  ;[1 1 1] Lock this token  (Keep it)
  (Variables|Default|SetLockedCross true))

(event EventBeginPlay
  ;[1 1 1] Binding dispatchers
  (bind _returnvalue (Actor|GetActorOfClass "/Game/ThirdPersonBP/Blueprints/ThirdPersonGameMode.ThirdPersonGameMode_C"))
  (EventDispatchers|BindEventtoDestroyTokenDispatcher _returnvalue (delegate Custom|Destroy%20Token))
  (EventDispatchers|BindEventtoLockToken (delegate Custom|Lock%20This%20token))
  (Utilities|FlowControl|Delay 2.0)
  (Audio|PlaySoundatLocation "/Game/SFX/big-impactwav-7054.big-impactwav-7054" (Transformation|GetActorLocation) "0, 0, 0" 1.0 1.0 0.0 0 0 0))

(fn ConstructionScript)