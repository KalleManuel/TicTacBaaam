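; BP_TokenDounot is a donut token actor that can be destroyed by a game-wide event unless it has been locked.
; On BeginPlay it binds to the destroy dispatcher on ThirdPersonGameMode and to its own LockToken dispatcher, then plays a delayed impact sound.
; Locking sets a flag that makes the token ignore destruction.
; An unlocked token spawns an explosion effect and sound, then destroys itself.
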(event Custom|Destroy%20Token
  (bind _returnvalue (Transformation|GetActorLocation))
  (if (not (Variables|Default|GetLockedDonout))
    (Effects|SpawnEmitteratLocation "/Game/StarterContent/Particles/P_Explosion.P_Explosion" _returnvalue "0, 0, 0" "2.000000,2.000000,2.000000")
    (Audio|PlaySoundatLocation "/Game/StarterContent/Audio/Explosion02.Explosion02" _returnvalue "0, 0, 0" 1.0 1.0 0.0 0 0 0)
    (Actor|DestroyActor)))

(event Custom|Lock%20This%20token
  (Variables|Default|SetLockedDonout true))

(event EventBeginPlay
  (bind _returnvalue (Actor|GetActorOfClass "/Game/ThirdPersonBP/Blueprints/ThirdPersonGameMode.ThirdPersonGameMode_C"))
  (EventDispatchers|BindEventtoDestroyTokenDispatcher _returnvalue (delegate Custom|Destroy%20Token))
  (EventDispatchers|BindEventtoLockToken (delegate Custom|Lock%20This%20token))
  (Utilities|FlowControl|Delay 2.0)
  (Audio|PlaySoundatLocation "/Game/SFX/big-impactwav-7054.big-impactwav-7054" (Transformation|GetActorLocation) "0, 0, 0" 1.0 1.0 0.0 0 0 0))

(fn ConstructionScript)