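; BP_WinningCondition judges a colour-slot board game, checking predefined lines in WinningConditions for a win or draw.
; Winning compares adjacent slots, ignoring empty FloorSlot colour, and needs a first-pair match plus a later adjacent match.
; Draw increments DrawNine for lines containing both blue and green, firing when it equals nine; the counter is never reset here.
; Results trigger the game mode screen, music and player dollar stats, plus a character pose on wins.
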(fn ConstructionScript)

(fn Winning
  (for _array_element (Variables|Default|GetWinningConditions)
    (LocalVariables|SetMatchTwo false)
    (for (_array_element_2 _array_index) (.slot _array_element)
      (if (not (== _array_index 3))
        (if (== (Variables|/Game/BluePrints/BP_Slot.BP_Slot_C|Get%20TheColor _array_element_2) (Variables|/Game/BluePrints/BP_Slot.BP_Slot_C|Get%20TheColor (Utilities|Array|Get(acopy) (.slot _array_element) (+ _array_index 1))))
          (if (not (== (Variables|/Game/BluePrints/BP_Slot.BP_Slot_C|Get%20TheColor _array_element_2) "/Game/Materials/FloorSlot.FloorSlot"))
            (if (== _array_index 0)
              (LocalVariables|SetMatchTwo true)
              (elif (LocalVariables|GetMatchTwo)
                (bind _returnvalue (Actor|GetActorOfClass "/Game/ThirdPersonBP/Blueprints/ThirdPersonGameMode.ThirdPersonGameMode_C"))
                (Default|AddWinscreen _returnvalue)
                (bind _returnvalue_2 (Actor|GetActorOfClass "/Game/ThirdPersonBP/Blueprints/ThirdPersonCharacter.ThirdPersonCharacter_C"))
                (Default|WinPose _returnvalue_2)
                (bind _returnvalue_3 (Actor|GetActorOfClass "/Game/BluePrints/GameMusic.GameMusic_C"))
                (Default|WonGame _returnvalue_3)
                (bind _returnvalue_4 (Actor|GetActorOfClass "/Game/BluePrints/BP_PlayerStats.BP_PlayerStats_C"))
                (Default|WinDollar _returnvalue_4)
                (return true))))))))
  (return false))

(fn Draw
  (for _array_element (Variables|Default|GetWinningConditions)
    (Variables|Default|SetBlue false)
    (Variables|Default|SetGreen false)
    (for _array_element_2 (.slot _array_element)
      (if (== (Variables|/Game/BluePrints/BP_Slot.BP_Slot_C|Get%20TheColor _array_element_2) "/Game/Materials/ShinyBlue.ShinyBlue")
        (Variables|Default|SetBlue true)
        (elif (== (Variables|/Game/BluePrints/BP_Slot.BP_Slot_C|Get%20TheColor _array_element_2) "/Game/Materials/ShinyGreen.ShinyGreen")
          (Variables|Default|SetGreen true))))
    (if (Variables|Default|GetBlue)
      (if (Variables|Default|GetGreen)
        (Math|Integer|IncrementInt (Variables|Default|GetDrawNine)))))
  (if (== (Variables|Default|GetDrawNine) 9)
    (bind _returnvalue (Actor|GetActorOfClass "/Game/BluePrints/BP_PlayerStats.BP_PlayerStats_C"))
    (Default|DrawDollar _returnvalue)
    (bind _returnvalue_2 (Actor|GetActorOfClass "/Game/ThirdPersonBP/Blueprints/ThirdPersonGameMode.ThirdPersonGameMode_C"))
    (Default|AddDrawScreen _returnvalue_2)
    (bind _returnvalue_3 (Actor|GetActorOfClass "/Game/BluePrints/GameMusic.GameMusic_C"))
    (Default|WonGame _returnvalue_3)
    (return true)))